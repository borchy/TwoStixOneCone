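; RotationCharacter is a character Blueprint that handles automatic fire of bullets or grenades.
; Primary and secondary fire inputs set the projectile class, then share a Gate that loops through a short Delay to repeat shots while held.
; Releasing either input closes the shared Gate.
; FireProjectile spawns the half-scale projectile just ahead of the actor along its facing and plays a pitched-up laser sound.
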(event `InputAction|Primary Fire`
  (:`Pressed`
    (set `self.Projectile` "/Game/Blueprints/Bullet.Bullet_C")
    (`|ExecutionSequence` :!label _label
      (:`then_0`
        (goto _label_2 :!via `Open`))
      (:`then_1`
        (`/Engine/EditorBlueprintResources/StandardMacros.Gate` true :!label _label_2
          (:`Exit`
            (`self.Fire Projectile` (`self.Projectile`))
            (`KismetSystemLibrary.Delay` 0.2)
            (goto _label_2))))))
  (:`Released`
    (goto _label_2 :!via `Close`)))

(event `InputAction|Secondary Fire`
  (:`Pressed`
    (set `self.Projectile` "/Game/Blueprints/Grenade.Grenade_C")
    (goto _label))
  (:`Released`
    (goto _label_2 :!via `Close`)))

(fn `Fire Projectile`
  (params (Projectile :type "Actor Class Reference"))
  (bind _returnvalue (`self.K2_GetActorRotation`))
  (`|SpawnActorFromClass` Projectile (`KismetMathLibrary.MakeTransform` (+ (* (`KismetMathLibrary.GetForwardVector` _returnvalue) 20.0) (`self.K2_GetActorLocation`)) _returnvalue (`KismetMathLibrary.MakeVector` 0.5 0.5 0.5)) true)
  (`GameplayStatics.PlaySoundAtLocation` "/Game/StarterContent/Audio/Laser_Cannon-Mike_Koenig-797224747.Laser_Cannon-Mike_Koenig-797224747" (`self.K2_GetActorLocation`) 1.0 1.5 0.75))

(fn `UserConstructionScript`)