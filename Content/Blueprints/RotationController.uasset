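; RotationController is a controller Blueprint that turns its pawn toward the mouse cursor and moves it from axis input.
; Every tick it sets the pawn's yaw toward the deprojected mouse world location, zeroing pitch and roll, with no trace against the scene.
; MoveForward and MoveRight add movement along world X and Y, so movement is independent of facing.
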(event `self.ReceiveTick`
  (params (DeltaSeconds :type "Float (single-precision)"))
  (bind _returnvalue (`self.K2_GetPawn`))
  ;[1 1 1] Mouse Rotation
  (`self.SetActorRotation` _returnvalue (`KismetMathLibrary.MakeRot` 0.0 (.yaw (`KismetMathLibrary.FindLookAtRotation` (`self.K2_GetActorLocation` _returnvalue) (`self.DeprojectMousePositionToWorld`))))))

(event `InputAxis|MoveForward`
  (params (AxisValue :type "Float (single-precision)"))
  ;[1 1 1] Keboard Movement
  (`Pawn.AddMovementInput` (`self.K2_GetPawn`) (1.0 0.0 0.0) AxisValue false))

(event `InputAxis|MoveRight`
  (params (AxisValue :type "Float (single-precision)"))
  ;[1 1 1] Keboard Movement
  (`Pawn.AddMovementInput` (`self.K2_GetPawn`) (0.0 1.0 0.0) AxisValue false))

(fn `UserConstructionScript`)