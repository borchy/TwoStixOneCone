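; Behavior tree task that makes an AI-controlled enemy shoot bullets at the actor stored in a blackboard key.
; On every tick it passes the controlled pawn and target to FireAt, with no cooldown and no finish call.
; FireAt spawns a Bullet slightly ahead of the pawn toward the target, at a fixed world height, rotated only in yaw.
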(event `self.ReceiveTick`
  (params (OwnerActor :type "Actor Object Reference") (DeltaSeconds :type "Float (single-precision)"))
  (bind _asaicontroller (cast `AIController` OwnerActor))
  (`self.FireAt` (`Controller.K2_GetPawn` _asaicontroller) (`BTFunctionLibrary.GetBlackboardValueAsActor` (`self.TargetKey`))))

(fn `FireAt`
  (params (CurrentActor :type "Actor Object Reference") (TargetActor :type "Actor Object Reference"))
  (bind _returnvalue (`Actor.K2_GetActorLocation` CurrentActor))
  (bind _returnvalue_2 (`KismetMathLibrary.MakeVector` (.x (+ _returnvalue (* (`KismetMathLibrary.Normal` (`self.DirectionVector`)) 10.0))) (.y (+ _returnvalue (* (`KismetMathLibrary.Normal` (`self.DirectionVector`)) 10.0))) 100.0))
  (set `self.DirectionVector` (- (`Actor.K2_GetActorLocation` TargetActor) _returnvalue))
  (`|SpawnActorFromClass` "/Game/Blueprints/Bullet.Bullet_C" (`KismetMathLibrary.MakeTransform` _returnvalue_2 (`KismetMathLibrary.MakeRot` 0.0 (.yaw (`KismetMathLibrary.FindLookAtRotation` _returnvalue _returnvalue_2))))))