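; Behavior Tree service for enemy AI that records the distance between the controlled pawn and a target actor in the Blackboard.
; On each tick it casts the owner to an AIController and reads the actor stored under TargetKey.
; It writes the straight-line distance between the two locations to DistanceKey, or zero when the target is invalid.
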(event `self.ReceiveTick`
  (params (OwnerActor :type "Actor Object Reference") (DeltaSeconds :type "Float (single-precision)"))
  (bind _returnvalue (`BTFunctionLibrary.GetBlackboardValueAsActor` (`self.TargetKey`)))
  (bind _asaicontroller (cast `AIController` OwnerActor))
  (`/Engine/EditorBlueprintResources/StandardMacros.IsValid` _returnvalue
    (:`Is Valid`
      (`BTFunctionLibrary.SetBlackboardValueAsFloat` (`self.DistanceKey`) (`KismetMathLibrary.VSize` (- (`Actor.K2_GetActorLocation` (`Controller.K2_GetPawn` _asaicontroller)) (`Actor.K2_GetActorLocation` _returnvalue)))))
    (:`Is Not Valid`
      (`BTFunctionLibrary.SetBlackboardValueAsFloat` (`self.DistanceKey`)))))