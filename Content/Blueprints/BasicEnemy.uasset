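; BasicEnemy is an enemy actor that takes damage and is destroyed when its hit points run out.
; AnyDamage subtracts damage from HitPoints, then flashes the Body with a hit material before restoring the base Material after a short delay.
; The construction script sets the Body's mesh from a variable and applies a dynamic material instance created from Material, which the hit flash later replaces with the plain Material.
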(event `self.ReceiveAnyDamage`
  (params (Damage :type "Float (single-precision)") (DamageType :type "DamageType Object Reference") (InstigatedBy :type "Controller Object Reference") (DamageCauser :type "Actor Object Reference"))
  (`|ExecutionSequence`
    (:`then_0`
      (set `self.HitPoints` (- (`self.HitPoints`) Damage))
      (if (<= (`self.HitPoints`) 0.0)
        (`self.K2_DestroyActor`)))
    (:`then_1`
      (`PrimitiveComponent.SetMaterial` (`self.Body`) 0 "/Game/Materials/M_EnemyHit.M_EnemyHit")
      (`KismetSystemLibrary.Delay` 0.2)
      (`PrimitiveComponent.SetMaterial` (`self.Body`) 0 (`self.Material`)))))

(fn `UserConstructionScript`
  (`StaticMeshComponent.SetStaticMesh` (`self.Body`) (`self.Mesh`))
  (bind _returnvalue (`KismetMaterialLibrary.CreateDynamicMaterialInstance` (`self.Material`)))
  (`PrimitiveComponent.SetMaterial` (`self.Body`) 0 _returnvalue))